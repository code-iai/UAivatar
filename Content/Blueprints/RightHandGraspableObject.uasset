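; Actor that the ThirdPersonAvatar can grasp with its right hand.
; On overlap, if right-hand IK is active and grasping is allowed, it snaps to hand_rSocket with a fixed mesh offset, disables physics and collision, and flags the avatar as grasping.
; DetachFromCharacter releases it, restores physics and collision, and uses a short timer before re-enabling grasping to prevent immediate re-pickup.
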(event `self.ReceiveBeginPlay`
  ;[1 1 1] Initialization
  (set `self.IsGrasped` false)
  (set `self.CanGrasp` true))

(event `self.ReceiveActorBeginOverlap`
  (params (OtherActor :type "Actor Object Reference"))
  (bind _staticmesh (`self.StaticMesh`))
  (bind _asthird_person_avatar (cast `/UIAIAvatar/Blueprints/ThirdPersonAvatar` OtherActor))
  (`KismetSystemLibrary.PrintString` "")
  (if (and (`IAIAvatarCharacter.IKEnableActive_r` _asthird_person_avatar) (`self.CanGrasp`))
    (if (not (`self.IsGrasped`))
      (`KismetSystemLibrary.PrintString` "")
      ;[1 1 1] Attaching the Object to a Character
      (`self.K2_AttachToComponent` (`Character.Mesh` _asthird_person_avatar) "hand_rSocket" "SnapToTarget" "SnapToTarget" "KeepWorld")
      (`PrimitiveComponent.SetSimulatePhysics` _staticmesh false)
      (`SceneComponent.K2_SetRelativeLocationAndRotation` _staticmesh (-1.0 2.0 5.0) (struct :`Pitch` 108.0 :`Roll` 75.0) false false)
      (set `self.IsGrasped` true)
      (set `self.CanGrasp` false)
      (set `IAIAvatarCharacter.isGrasped_r` true _asthird_person_avatar)
      (`self.SetActorEnableCollision` false))))

(fn `DetachFromCharacter`
  (`KismetSystemLibrary.PrintString` "")
  (`self.K2_DetachFromActor` "KeepWorld" "KeepWorld" "KeepWorld")
  (set `self.IsGrasped` false)
  (`PrimitiveComponent.SetSimulatePhysics` (`self.StaticMesh`) true)
  (`self.SetActorEnableCollision` true)
  (`KismetSystemLibrary.K2_SetTimer` null "ReactivateCanGrasp" 2.0))

(fn `ReactivateCanGrasp`
  (set `self.CanGrasp` true)
  (`KismetSystemLibrary.PrintString` ""))

(fn `UserConstructionScript`)