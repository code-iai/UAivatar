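; A physics prop that an IAI avatar character grasps in its left hand when it overlaps the object while the avatar's IK is active.
; Grasping attaches it to the left-hand socket, turns off physics and collision, and sets the animation instance's left-hand grasping alpha.
; DetachFromCharacter releases it in place, restores physics and collision, and starts a short timer before it can be grasped again.
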(event `self.ReceiveBeginPlay`
  ;[1 1 1] Initialization
  (set `self.IsGrasped` false)
  (set `self.CanGrasp` true))

(event `self.ReceiveActorBeginOverlap`
  (params (OtherActor :type "Actor Object Reference"))
  (bind _staticmesh (`self.StaticMesh`))
  (bind _asiaiavatar_character (cast `IAIAvatarCharacter` OtherActor))
  (`KismetSystemLibrary.PrintString` "")
  (if (and (`IAIAvatarCharacter.IKEnableActive` _asiaiavatar_character) (`self.CanGrasp`))
    (if (not (`self.IsGrasped`))
      (`KismetSystemLibrary.PrintString` "")
      ;[1 1 1] Attaching the Object to a Character
      (`self.K2_AttachToComponent` (`Character.Mesh` _asiaiavatar_character) "hand_lSocket" "SnapToTarget" "KeepRelative" "KeepWorld")
      (`PrimitiveComponent.SetSimulatePhysics` _staticmesh false)
      (`SceneComponent.K2_SetRelativeLocationAndRotation` _staticmesh (0.0 5.0 0.0) (struct :`Pitch` 190.0) false false)
      (set `self.IsGrasped` true)
      (set `self.CanGrasp` false)
      (bind _asiaiavatar_animation_instance (cast `IAIAvatarAnimationInstance` (`SkeletalMeshComponent.GetAnimInstance` (`Character.Mesh` _asiaiavatar_character))))
      (set `IAIAvatarAnimationInstance.leftHandGraspingAlpha` 1.0 _asiaiavatar_animation_instance)
      (`self.SetActorEnableCollision` false))))

(fn `DetachFromCharacter`
  (`KismetSystemLibrary.PrintString` "")
  (`self.K2_DetachFromActor` "KeepWorld" "KeepWorld" "KeepWorld")
  (set `self.IsGrasped` false)
  (`PrimitiveComponent.SetSimulatePhysics` (`self.StaticMesh`) true)
  (`self.SetActorEnableCollision` true)
  (`KismetSystemLibrary.K2_SetTimer` null "ReactivateCanGrasp" 2.0))

(fn `ReactivateCanGrasp`
  (set `self.CanGrasp` true)
  (`KismetSystemLibrary.PrintString` ""))

(fn `UserConstructionScript`)